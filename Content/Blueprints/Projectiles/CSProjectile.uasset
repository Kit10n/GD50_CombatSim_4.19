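; CSProjectile is a projectile that resolves bullet or explosive impacts on component hit, then destroys itself.
; It scales bullet damage by distance from its spawn point and plays impact sound, with decals on non-CSCharacter hits.
; Explosive rounds apply radial damage and VFX.
; Bullets spawn particles, skip the instigator and living characters of the instigator's class, and push dead characters with a bone impulse.
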(event `self.ProjectileCollision.OnComponentHit`
  (params (HitComponent :type "PrimitiveComponent Object Reference") (OtherActor :type "Actor Object Reference") (OtherComp :type "PrimitiveComponent Object Reference") (NormalImpulse :type "Vector Structure") (Hit :type "HitResult Structure (by ref)"))
  (bind (_bblockinghit _binitialoverlap _time _distance _location _impactpoint _normal _impactnormal _physmat _hitactor _hitcomponent _hitbonename) (`GameplayStatics.BreakHitResult` Hit))
  ;[1 1 1] Hit event
  (set `self.HitActor` OtherActor)
  (set `self.HitLocation` _location)
  (set `self.ImpactNormal` _impactnormal)
  (set `self.HitBoneName` _hitbonename)
  ;[1 1 1] Damage fall off
  (set `self.Damage` (`KismetMathLibrary.MapRangeUnclamped` (`KismetMathLibrary.FClamp` (`KismetMathLibrary.VSize` (- (`self.StartLocation`) (`self.HitLocation`))) (`self.DamageFalloffDistanceMin`) (`self.DamageFalloffDistanceMax`)) (`self.DamageFalloffDistanceMin`) (`self.DamageFalloffDistanceMax`) (`self.Damage`) (`self.DamageFalloffModMax`)))
  ;[1 1 1] Decal
  (cast `/Game/Blueprints/Characters/CSCharacter` (`self.HitActor`)
    (:`then`
      _)
    (:`CastFailed`
      (`GameplayStatics.SpawnDecalAtLocation` (`self.ImpactDecalMaterial`) (`self.ImpactDecalSize`) (`self.HitLocation`) (`KismetMathLibrary.Conv_VectorToRotator` (`self.ImpactNormal`)) (`self.ImpactDecalLifeSpan`))))
  (cast `Character` (`self.HitActor`)
    (:`then`
      (set `self.ImpactSFX` "/Game/Weapons/AssaultRifle/Audio/Rifle_BulletImpact_Cue.Rifle_BulletImpact_Cue"))
    (:`CastFailed`
      _))
  (`GameplayStatics.PlaySoundAtLocation` (`self.ImpactSFX`) (`self.HitLocation`))
  (if (`self.Explosive`)
    ;[1 1 1] Explosive Damage
    (`GameplayStatics.ApplyRadialDamageWithFalloff` :`BaseDamage` (`self.ExplosiveDamage`) :`MinimumDamage` (`self.MinimumExplosiveDamage`) :`Origin` (`self.HitLocation`) :`DamageInnerRadius` (`self.ExplosiveDamageInnerRadius`) :`DamageOuterRadius` (`self.ExplosiveDamageOuterRadius`) :`DamageFalloff` 1.0 :`DamageTypeClass` (`self.ExplosiveDamageType`) :`DamageCauser` self :`InstigatedByController` (`self.GetInstigatorController`) :`DamagePreventionChannel` "ECC_WorldStatic")
    ;[1 1 1] MICHAEL BAY
    (`GameplayStatics.SpawnEmitterAtLocation` (`self.ExplosiveVFX`) (`self.HitLocation`) (`KismetMathLibrary.Conv_VectorToRotator` (`self.ImpactNormal`)))
    (else
      ;[1 1 1] Dont shoot ourselvs
      (if (!= (`self.HitActor`) (`self.GetInstigator`))
        ;[1 1 1] Particle
        (`GameplayStatics.SpawnEmitterAtLocation` (`self.ImpactVFX`) (`self.HitLocation`) (`KismetMathLibrary.Conv_VectorToRotator` (`self.ImpactNormal`)) (select `bool` (== (`GameplayStatics.GetObjectClass` (`self.HitActor`)) "/Game/Blueprints/Characters/CSCharacter_Player.CSCharacter_Player_C") :`false` (1.0 1.0 1.0) :`true` (0.5 0.5 0.5) :!type "Vector Structure"))
        ;[1 1 1] Avoid friendly fire
        (if (== (`GameplayStatics.GetObjectClass` (`self.GetInstigator`)) (`GameplayStatics.GetObjectClass` (`self.HitActor`)))
          (bind _ascscharacter (cast `/Game/Blueprints/Characters/CSCharacter` (`self.HitActor`))
            (:`then`
              (if (<= (`/Game/Blueprints/Characters/CSCharacter.Health` _ascscharacter) 0.0)
                ;[1 1 1] Bullet Damage
                (`GameplayStatics.ApplyDamage` (`self.HitActor`) (`self.Damage`) (`self.GetInstigatorController`) self (`self.ProjectileDamageType`) :!label _label)
                ;[1 1 1] Impulse
                (bind _ascscharacter_2 (cast `/Game/Blueprints/Characters/CSCharacter` (`self.HitActor`))
                  (:`then`
                    (if (<= (`/Game/Blueprints/Characters/CSCharacter.Health` _ascscharacter_2) 0.0)
                      (bind _output_get (set `self.ImpulseVector` (* (`KismetMathLibrary.Normal` (`KismetMathLibrary.Conv_RotatorToVector` (`self.K2_GetActorRotation`))) (`self.ImpulseForce`))))
                      (`PrimitiveComponent.AddImpulse` (`Character.Mesh` _ascscharacter_2) _output_get (`self.HitBoneName`) false)))
                  (:`CastFailed`
                    _))))
            (:`CastFailed`
              _))
          (else
            (goto _label)))
        (else
          (`KismetSystemLibrary.PrintString` "Projectile hit self, destroyed" false)))))
  ;[1 1 1] Destroy self
  (`self.K2_DestroyActor`))

(fn `UserConstructionScript`
  (set `self.StartLocation` (`self.K2_GetActorLocation`)))