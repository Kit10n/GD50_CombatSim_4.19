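; AI controller for enemies that runs the CSBTEnemy behavior tree on possession, starting in the Scripted state.
; Perception updates switch it to Systemic once the player pawn is within range, then target the sensed player character or a player controller's pawn.
; A new target is written to the blackboard, focused, announced with a sound and reported through CallPlayerSpotted.
; Helper functions also push AI state and patrol path to the blackboard.
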(event `self.OnPossess`
  (params (PossessedPawn :type "Pawn Object Reference"))
  ;[1 1 1] Begin possesion, start behavior tree
  (`self.RunBehaviorTree` "/Game/AI/CSBTEnemy.CSBTEnemy")
  (`self.SetAIState` "NewEnumerator1"))

(event `self.AIPerception.OnPerceptionUpdated`
  (params (UpdatedActors :type "Array of Actor Object Reference (by ref)"))
  ;[1 1 1] Sensed the player
  (for _array_element UpdatedActors
    (switch `/Game/Blueprints/Characters/CSAIStates` (`self.AIState`)
      (:`NewEnumerator0`
        (bind _ascscharacter_player (cast `/Game/Blueprints/Characters/CSCharacter_Player` _array_element :!label _label)
          (:`then`
            (`self.SetTarget` _ascscharacter_player))
          (:`CastFailed`
            (bind _ascsplayer_controller (cast `/Game/Blueprints/Characters/CSPlayerController` _array_element))
            (`self.SetTarget` (`self.K2_GetPawn` _ascsplayer_controller)))))
      (:`NewEnumerator1`
        (if (< (`self.GetDistanceTo` (`self.K2_GetPawn`) (`GameplayStatics.GetPlayerPawn` 0)) 1000.0)
          (`self.SetAIState` "NewEnumerator0")
          (goto _label))))))

(fn `AssignPatrolPath`
  (params (NewPatrolPath :type "/Game/Blueprints/Ingredients/CSPatrolPath Object Reference"))
  (returns (Return :type Boolean))
  (locals (NewPatrolPathLocal :type "/Game/Blueprints/Ingredients/CSPatrolPath Object Reference"))
  (bind _output_get (set `local.NewPatrolPathLocal` NewPatrolPath))
  (`/Engine/EditorBlueprintResources/StandardMacros.IsValid` _output_get
    (:`Is Valid`
      (`BlackboardComponent.SetValueAsObject` (`AIBlueprintHelperLibrary.GetBlackboard` self) "PatrolPath" (`local.NewPatrolPathLocal`)))
    (:`Is Not Valid`
      _))
  ;[1 1 1] Return
  (return true))

(fn `SetAIState`
  (params (AIState :type "/Game/Blueprints/Characters/CSAIStates Enum" :default "NewEnumerator0"))
  (bind _output_get (set `self.AIState` AIState))
  (`BlackboardComponent.SetValueAsEnum` (`AIBlueprintHelperLibrary.GetBlackboard` self) "AIState" _output_get))

(fn `SetTarget`
  (params (NewActorTarget :type "Actor Object Reference"))
  (bind _returnvalue (`BlackboardComponent.GetValueAsObject` (`AIBlueprintHelperLibrary.GetBlackboard` self) "Target"))
  (`/Engine/EditorBlueprintResources/StandardMacros.IsValid` _returnvalue
    (:`Is Valid`
      (if (not (== _returnvalue NewActorTarget))
        (`BlackboardComponent.SetValueAsObject` (`AIBlueprintHelperLibrary.GetBlackboard` self) "Target" NewActorTarget :!label _label)
        (`GameplayStatics.PlaySoundAtLocation` "/Game/Audio/SFX/Ingredients/Blueprints_Scanner_Change05_Cue.Blueprints_Scanner_Change05_Cue" (`self.K2_GetActorLocation` (`self.K2_GetPawn`)))
        (`self.K2_SetFocus` NewActorTarget)
        (`self.PlayerSpotted` (`self.K2_GetActorLocation` NewActorTarget))))
    (:`Is Not Valid`
      (goto _label))))

(fn `UserConstructionScript`)