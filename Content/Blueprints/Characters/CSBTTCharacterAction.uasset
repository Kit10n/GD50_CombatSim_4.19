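; Behavior tree task that lets AI-controlled CSCharacter pawns perform a single character action, such as firing, ironsights, crouching, sprinting, reloading or jumping.
; On execute, it casts the controlled pawn to CSCharacter and switches on ActionToPerform to call the matching start or stop function.
; It finishes successfully right after the call without waiting for the action to complete, and fails if the pawn is invalid or not a CSCharacter.
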(event `self.ReceiveExecuteAI`
  (params (OwnerController :type "AIController Object Reference") (ControlledPawn :type "Pawn Object Reference"))
  (bind _character (`self.Character`))
  (`/Engine/EditorBlueprintResources/StandardMacros.IsValid` ControlledPawn
    (:`Is Valid`
      (bind _ascscharacter (cast `/Game/Blueprints/Characters/CSCharacter` ControlledPawn)
        (:`then`
          (set `self.Character` _ascscharacter)
          (switch `/Game/Blueprints/Characters/CSCharacterActions` (`self.ActionToPerform`)
            (:`NewEnumerator0`
              (`/Game/Blueprints/Characters/CSCharacter.StartFiring` _character))
            (:`NewEnumerator1`
              (`/Game/Blueprints/Characters/CSCharacter.StopFiring` _character))
            (:`NewEnumerator2`
              (`/Game/Blueprints/Characters/CSCharacter.StartIronsights` _character))
            (:`NewEnumerator3`
              (`/Game/Blueprints/Characters/CSCharacter.StopIronsights` _character))
            (:`NewEnumerator4`
              (`/Game/Blueprints/Characters/CSCharacter.StartCrouch` _character))
            (:`NewEnumerator5`
              (`/Game/Blueprints/Characters/CSCharacter.StopCrouch` _character))
            (:`NewEnumerator6`
              (`/Game/Blueprints/Characters/CSCharacter.StartSprint` _character))
            (:`NewEnumerator7`
              (`/Game/Blueprints/Characters/CSCharacter.StopSprint` _character))
            (:`NewEnumerator8`
              (`/Game/Blueprints/Characters/CSCharacter.StartReload` _character))
            (:`NewEnumerator9`
              (`/Game/Blueprints/Characters/CSCharacter.StartJump` _character)))
          (`self.FinishExecute` true))
        (:`CastFailed`
          (`self.FinishExecute` false :!label _label))))
    (:`Is Not Valid`
      (goto _label))))