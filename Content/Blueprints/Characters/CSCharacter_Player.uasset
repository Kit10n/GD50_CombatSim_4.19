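; Player character Blueprint that adds hit, low-health and death feedback on top of its parent character's health logic.
; The ModifyHealth override calls the parent, then scales low-health post-process weight by remaining health below a threshold.
; When health is not being added, it also plays a timeline-driven damage post-process and a camera shake.
; A death delegate bound on BeginPlay plays the mission-failed sound after a short delay.
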(event `self.ReceiveBeginPlay`
  (`parent.ReceiveBeginPlay`)
  ;[1 1 1] Mission failed sound
  (add `self.CharacterDied` (delegate `PlayerDied`)))

(event `PlayerDied`
  ;[1 1 1] Mission failed sound
  (`KismetSystemLibrary.Delay` 1.2)
  (`GameplayStatics.PlaySound2D` "/Game/Audio/SFX/TACCOM/SFX_MissionFailed_Cue.SFX_MissionFailed_Cue"))

(event `PlayHitFeedback`
  (bind (_direction _effectalpha) (`Timeline|DamageEffect` :!via `PlayFromStart`)
    (:`Update`
      (set `PostProcessComponent.BlendWeight` (`KismetMathLibrary.Lerp` 0.0 1.0 _effectalpha) (`self.DamagePostProcess`)))))

(fn `ModifyHealth`
  (params (Amount :type "Float (double-precision)") (DamageType :type "DamageType Object Reference") (InstigatedBy :type "Controller Object Reference") (DamageCauser :type "Actor Object Reference"))
  (returns (Health :type "Float (double-precision)") (AddHealth :type Boolean))
  (locals (AddingHealth :type Boolean :default false))
  (bind (_health _addhealth) (`parent.ModifyHealth` Amount DamageType InstigatedBy DamageCauser))
  ;[1 0.9542 0.165] Hit Feedback
  (set `local.AddingHealth` _addhealth)
  ;;[1 0.04688 0.04688] Low Health Post Process
  (set `PostProcessComponent.BlendWeight` (`KismetMathLibrary.Lerp` 1.0 0.0 (* (/ _health (`self.MaxHealth`)) (/ 1.0 (`self.LowHealthEffectThreshold`)))) (`self.LowHealthPostProcess`))
  (if (not (`local.AddingHealth`))
    ;;[0.1851 1 0.9403] Damage Post Process
    (`TimelineComponent.PlayFromStart` (`self.DamageEffect`))
    ;;[0.5533 0.2661 1] Camera Shake
    (`PlayerController.ClientStartCameraShake` :`self` (`GameplayStatics.GetPlayerController` 0) :`Shake` "/Game/Effects/CameraShake/CSCameraShake_Hit.CSCameraShake_Hit_C"))
  (return (`self.Health`) false))

(fn `UserConstructionScript`
  (`parent.UserConstructionScript`))