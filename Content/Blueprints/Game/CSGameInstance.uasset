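; Game instance that holds game-wide state for checkpoints, a music track switch and a security switch.
; SetCheckpoint stores a PlayerStart's tag, and GetCheckpoint searches the world's PlayerStarts for the matching one, so only the tag is kept rather than an actor reference.
; PlaySecondMusicTrack and DisableSecurity each set a state variable behind a DoOnce, without playing audio or touching actors themselves.
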(fn `DisableSecurity`
  (`/Engine/EditorBlueprintResources/StandardMacros.DoOnce` false
    (:`Completed`
      (set `self.V_Security` 1)
      (return))))

(fn `GetCheckpoint`
  (returns (CurrentPlayerStart :type "PlayerStart Object Reference"))
  (locals (CurrentCheckpointLocal :type "PlayerStart Object Reference"))
  (bind _outactors (`GameplayStatics.GetAllActorsOfClass` "/Script/Engine.PlayerStart"))
  (for _array_element _outactors
    (if (== (`PlayerStart.PlayerStartTag` _array_element) (`self.CurrentCheckpointTag`))
      (set `local.CurrentCheckpointLocal` _array_element)
      (break)))
  (return (`local.CurrentCheckpointLocal`)))

(fn `PlaySecondMusicTrack`
  (`/Engine/EditorBlueprintResources/StandardMacros.DoOnce` false
    (:`Completed`
      (set `self.V_MusicTrack` 1)
      (return))))

(fn `SetCheckpoint`
  (params (PlayerStart :type "PlayerStart Object Reference"))
  (returns (Return :type Boolean))
  (set `self.CurrentCheckpointTag` (`PlayerStart.PlayerStartTag` PlayerStart))
  (return true))