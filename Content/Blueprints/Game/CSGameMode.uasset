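; Game mode that runs a level's security system, objectives, player HUD and restarts.
; On BeginPlay it gathers all security ingredient actors, then relays enable, disable, trip and reset alarm changes to them by message and fires matching dispatchers.
; Player death, or a tripped alarm when that fail condition is set, reloads the level.
; Player start prefers Play-From-Here, then the GameInstance checkpoint; objective changes can play TACCOM audio.
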(event `self.EnableSecuritySystem`
  ;[1 1 1] Security system
  (if (not (`self.SecuritySystemEnabled`))
    (set `self.SecuritySystemEnabled` true)
    (set `self.AlarmTripped` false)
    (`self.OnSecuritySystemEnabled`)
    (for _array_element (`self.AllSecurityIngredients`)
      (message `/Game/Blueprints/Ingredients/CSSecurityInterface.EnableSecuritySystem` _array_element))))

(event `self.ReceiveBeginPlay`
  ;[1 1 1] Comment
  (bind _returnvalue (`GameplayStatics.GetCurrentLevelName` true))
  (`self.SetCurrentLevel` self (`KismetStringLibrary.Conv_StringToName` _returnvalue))
  ;[1 1 1] Create player UMG
  (bind _returnvalue_2 (`|CreateWidget` "/Game/UI/UMG/CSPlayerUMG.CSPlayerUMG_C" (`GameplayStatics.GetPlayerController` 0)))
  (bind _output_get (set `self.PlayerHUD` _returnvalue_2))
  (`UserWidget.AddToPlayerScreen` _output_get 0)
  ;[1 1 1] Reload level on player death
  (add `self.OnDestroyed` (`GameplayStatics.GetPlayerCharacter` 0) (delegate `RestartLevel`))
  ;[1 1 1] Security ingredients
  (bind _outactors (`GameplayStatics.GetAllActorsOfClass` "/Game/Blueprints/Ingredients/CSBaseSecurityIngredient.CSBaseSecurityIngredient_C"))
  (for _array_element _outactors
    (`KismetArrayLibrary.Array_AddUnique` (`self.AllSecurityIngredients`) _array_element))
  (`self.EnableSecuritySystem`))

(event `self.DisableSecuritySystem`
  ;[1 1 1] Security system
  (if (`self.SecuritySystemEnabled`)
    (set `self.AlarmTripped` false)
    (set `self.SecuritySystemEnabled` false)
    (`self.OnSecuritySystemDisabled`)
    (for _array_element (`self.AllSecurityIngredients`)
      (message `/Game/Blueprints/Ingredients/CSSecurityInterface.DisableSecuritySystem` _array_element))))

(event `RestartLevel` :!signature `self.OnDestroyed`
  (params (DestroyedActor :type "Actor Object Reference"))
  ;[1 1 1] Reload level on player death
  (`/Engine/EditorBlueprintResources/StandardMacros.DoOnce` false
    (:`Completed`
      (`KismetSystemLibrary.Delay` 2.0)
      (`GameplayStatics.OpenLevel` (`self.CurrentLevel`)))))

(event `self.TripAlarm`
  (params (NewTarget :type "Actor Object Reference"))
  ;[1 1 1] Security system
  (set `self.SecurityAlarmTarget` NewTarget)
  (if (and (not (`self.AlarmTripped`)) (`self.SecuritySystemEnabled`))
    (set `self.AlarmTripped` true)
    (for _array_element (`self.AllSecurityIngredients`)
      (message `/Game/Blueprints/Ingredients/CSSecurityInterface.TripAlarm` _array_element (`self.SecurityAlarmTarget`)))
    (`self.OnAlarmTripped`)
    ;;[1 1 1] Fail if the security alarm goes off
    (if (`self.FailOnAlarmTripped`)
      (`/Engine/EditorBlueprintResources/StandardMacros.DoOnce` false
        (:`Completed`
          (`self.RestartLevel` null))))))

(event `self.ResetAlarm`
  ;[1 1 1] Security system
  (if (and (`self.SecuritySystemEnabled`) (`self.AlarmTripped`))
    (set `self.AlarmTripped` false)
    (`self.OnAlarmReset`)
    (for _array_element (`self.AllSecurityIngredients`)
      (message `/Game/Blueprints/Ingredients/CSSecurityInterface.ResetAlarm` _array_element))))

(fn `ChoosePlayerStart`
  (params (Player :type "Controller Object Reference"))
  (returns (ReturnValue :type "Actor Object Reference"))
  (locals (PlayerLocal :type "Controller Object Reference") (PlayerStartLocal :type "Actor Object Reference"))
  (bind _output_get (set `local.PlayerLocal` Player))
  (bind _returnvalue (`parent.ChoosePlayerStart` _output_get))
  (bind _asplayer_start_pie (cast `PlayerStartPIE` _returnvalue)
    (:`then`
      (return _asplayer_start_pie))
    (:`CastFailed`
      (bind _currentplayerstart (message `/Game/Blueprints/Game/CSCheckpointInterface.GetCheckpoint` (`GameplayStatics.GetGameInstance`)))
      (bind _output_get_2 (set `local.PlayerStartLocal` _currentplayerstart))
      (`/Engine/EditorBlueprintResources/StandardMacros.IsValid` _output_get_2
        (:`Is Valid`
          _)
        (:`Is Not Valid`
          (bind _returnvalue_2 (`parent.ChoosePlayerStart` (`local.PlayerLocal`)))
          (set `local.PlayerStartLocal` _returnvalue_2)))
      (return (`local.PlayerStartLocal`)))))

(fn `ClearObjective`
  (params (ObjectiveMarkerActor :type "Actor Object Reference") (PlayTACCOMAudio :type Boolean) (ObjectiveSuccess :type Boolean))
  (returns (Return :type Boolean))
  (locals (ObjectiveMarkerActorLocal :type "Actor Object Reference") (CurrentObjectiveIndexLocal :type "/Game/Blueprints/Game/CSObjectives Structure") (PlayTACCOMAudioLocal :type Boolean) (ObjectiveSuccessLocal :type Boolean))
  (set `local.ObjectiveMarkerActorLocal` ObjectiveMarkerActor)
  (set `local.PlayTACCOMAudioLocal` PlayTACCOMAudio)
  (set `local.ObjectiveSuccessLocal` ObjectiveSuccess)
  (for _array_element (`self.Objectives`)
    (bind _output_get (set `local.CurrentObjectiveIndexLocal` _array_element))
    (if (== (`.ObjectiveActor_4_97EA34D745469AABA2ABA89CB9314951` (break `/Game/Blueprints/Game/CSObjectives` _output_get)) (`local.ObjectiveMarkerActorLocal`))
      (`KismetArrayLibrary.Array_RemoveItem` (`self.Objectives`) (`local.CurrentObjectiveIndexLocal`))
      (if (`local.PlayTACCOMAudioLocal`)
        (`GameplayStatics.PlaySound2D` (select `bool` (`local.ObjectiveSuccessLocal`) :`false` "/Game/Audio/SFX/TACCOM/SFX_ObjectiveComplete_Cue.SFX_ObjectiveComplete_Cue" :`true` "/Game/Audio/SFX/TACCOM/SFX_ObjectiveComplete_Cue.SFX_ObjectiveComplete_Cue" :!type "SoundBase Object Reference"))
        (break)
        (else
          (break)))))
  (return true))

(fn `GetAllSecurityIngredients`
  (returns (Ingredients :type "Array of Actor Object Reference"))
  (return (`self.AllSecurityIngredients`)))

(fn `GetObjectives`
  (returns (Objectives :type "Array of /Game/Blueprints/Game/CSObjectives Structure"))
  (return (`self.Objectives`)))

(fn `Scene capture activation`
  (params (Activation :type Boolean))
  (returns (`Capture texture` :type "TextureRenderTarget2D Object Reference"))
  (return null))

(fn `SetAllSecurityIngredients`
  (returns (Return :type Boolean))
  (bind _outactors (`GameplayStatics.GetAllActorsOfClass` "/Game/Blueprints/Ingredients/CSSecurityAlarm.CSSecurityAlarm_C"))
  (for _array_element _outactors
    (`KismetArrayLibrary.Array_AddUnique` (`self.AllSecurityIngredients`) _array_element))
  (bind _outactors_2 (`GameplayStatics.GetAllActorsOfClass` "/Game/Blueprints/Ingredients/CSSecurityCamera.CSSecurityCamera_C"))
  (for _array_element_2 _outactors_2
    (`KismetArrayLibrary.Array_AddUnique` (`self.AllSecurityIngredients`) _array_element_2))
  (bind _outactors_3 (`GameplayStatics.GetAllActorsOfClass` "/Game/Blueprints/Ingredients/CSSecurityDoor.CSSecurityDoor_C"))
  (for _array_element_3 _outactors_3
    (`KismetArrayLibrary.Array_AddUnique` (`self.AllSecurityIngredients`) _array_element_3))
  (return false))

(fn `SetCurrentLevel`
  (params (CurrentLevel :type Name))
  (returns (Return :type Boolean))
  (locals (CurrentLevelLocal :type Name))
  (bind _output_get (set `local.CurrentLevelLocal` CurrentLevel))
  (set `self.CurrentLevel` _output_get)
  (return true))

(fn `SetFailConditions`
  (params (FailOnAlarmTripped :type Boolean))
  (returns (Return :type Boolean))
  (set `self.FailOnAlarmTripped` FailOnAlarmTripped)
  (return true))

(fn `SetObjective`
  (params (ObjectiveType :type "/Game/Blueprints/Game/CSObjectiveType Enum" :default "NewEnumerator0") (ObjectiveMarkerActor :type "Actor Object Reference") (PlayTACCOMAudio :type Boolean))
  (returns (Return :type Boolean))
  (locals (ObjectiveTypeLocal :type "/Game/Blueprints/Game/CSObjectiveType Enum") (ObjectiveMarkerActorLocal :type "Actor Object Reference") (PlayTACCOMAudioLocal :type Boolean))
  (set `local.ObjectiveTypeLocal` ObjectiveType)
  (set `local.ObjectiveMarkerActorLocal` ObjectiveMarkerActor)
  (set `local.PlayTACCOMAudioLocal` PlayTACCOMAudio)
  (`KismetArrayLibrary.Array_AddUnique` (`self.Objectives`) (make `/Game/Blueprints/Game/CSObjectives` (`local.ObjectiveTypeLocal`) (`local.ObjectiveMarkerActorLocal`)))
  (if (`local.PlayTACCOMAudioLocal`)
    (`GameplayStatics.PlaySound2D` (select `/Game/Blueprints/Game/CSObjectiveType` (`local.ObjectiveTypeLocal`) :`NewEnumerator0` "/Game/Audio/SFX/TACCOM/SFX_ReachTheTargetLocation_Cue.SFX_ReachTheTargetLocation_Cue" :`NewEnumerator1` "/Game/Audio/SFX/TACCOM/SFX_AssaultTheSector_Cue.SFX_AssaultTheSector_Cue" :`NewEnumerator2` "/Game/Audio/SFX/TACCOM/SFX_InfiltrateTheSector_Cue.SFX_InfiltrateTheSector_Cue" :`NewEnumerator3` "/Game/Audio/SFX/TACCOM/SFX_DefendTheTargetLocation_Cue.SFX_DefendTheTargetLocation_Cue" :!type "SoundBase Object Reference")))
  (return true))

(fn `UserConstructionScript`)