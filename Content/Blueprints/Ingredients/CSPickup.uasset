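; Pickup actor that grants a player either weapon ammo or a new weapon when walked over.
; SetUpPickup picks mesh, sound, clip amount or weapon class from pickup and weapon type, at construction or on a runtime type change.
; PickedUp succeeds only if the matching inventory slot has clip room or lacks a weapon, spawning weapons as needed.
; Success plays a sound and a cut-plane dissolve across the mesh bounds before destroying the actor.
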(event `self.PickupCollision.OnComponentBeginOverlap`
  (params (OverlappedComponent :type "PrimitiveComponent Object Reference") (OtherActor :type "Actor Object Reference") (OtherComp :type "PrimitiveComponent Object Reference") (OtherBodyIndex :type Integer) (bFromSweep :type Boolean) (SweepResult :type "HitResult Structure (by ref)"))
  ;[1 1 1] Player walks over the pickup
  (bind _ascscharacter_player (cast `/Game/Blueprints/Characters/CSCharacter_Player` OtherActor))
  (`/Engine/EditorBlueprintResources/StandardMacros.DoOnce` false :!label _label
    (:`Completed`
      (set `self.Character` _ascscharacter_player)
      (bind _successfullypickedup (`self.PickedUp`))
      (if _successfullypickedup
        ;[1 1 1] Set which direction the disolve should play in
        (bind (_min _max) (`self.GetPickupMeshWorldBounds`))
        (`MaterialInstanceDynamic.SetVectorParameterValue` (`self.DynamicMaterial`) "CutRotation" (`KismetMathLibrary.Conv_VectorToLinearColor` (`KismetMathLibrary.Conv_RotatorToVector` (`KismetMathLibrary.FindLookAtRotation` _max _min))))
        ;[1 1 1] Disolve animation
        (bind (_direction _0_1) (`Timeline|DisolvePickedUpTimeline`)
          (:`Update`
            (bind (_min_2 _max_2) (`self.GetPickupMeshWorldBounds`))
            (`MaterialInstanceDynamic.SetVectorParameterValue` (`self.DynamicMaterial`) "CutPlane" (`KismetMathLibrary.Conv_VectorToLinearColor` (`KismetMathLibrary.VLerp` _min_2 _max_2 _0_1))))
          (:`Finished`
            (`self.K2_DestroyActor`)))
        (else
          (goto _label :!via `Reset`))))))

(event `ChangePickupType`
  (params (PickupType :type "/Game/Blueprints/Ingredients/CSInventoryItemType Enum" :default "NewEnumerator0") (WeaponType :type "/Game/Blueprints/Ingredients/CSAmmoPickupType Enum" :default "NewEnumerator0"))
  ;[1 1 1] Player walks over the pickup
  ;;[1 0.5874 0.3636] Allows changing pickup type on runtime
  (set `self.PickupType` PickupType)
  (set `self.WeaponType` WeaponType)
  (`self.SetUpPickup` PickupType WeaponType))

(fn `GetPickupMeshWorldBounds`
  (returns (Min :type "Vector Structure") (Max :type "Vector Structure"))
  (bind _returnvalue (`self.K2_GetActorLocation`))
  (bind (_min _max) (`StaticMeshComponent.GetLocalBounds` (`self.PickupMesh`)))
  (return (+ _returnvalue _min) (+ _returnvalue _max)))

(fn `PickedUp`
  (returns (SuccessfullyPickedUp :type Boolean))
  (locals (SuccessfullyPickedUpLocal :type Boolean))
  (switch `/Game/Blueprints/Ingredients/CSInventoryItemType` (`self.PickupType`)
    (:`NewEnumerator0`
      ;[1 1 1] Check if we have the weapon this ammo is for
      (for _array_element (`/Game/Blueprints/Characters/CSCharacter.WeaponInventory` (`self.Character`))
        (bind (_weaponname _weapontype _weaponinstance _clipscurrent _clipsmax) (break `/Game/Blueprints/Characters/CSWeaponInventory` _array_element))
        ;;[1 1 1] Ensure we can add more ammo of this type
        (if (and (`|EnumEquality` (`self.WeaponType`) _weapontype) (< _clipscurrent _clipsmax))
          ;[1 1 1] Add ammo to inventory
          (`/Game/Blueprints/Characters/CSCharacter.ModifyInventory` (`self.Character`) "NewEnumerator0" "NewEnumerator0" (`self.WeaponType`) null (`self.ClipAmount`))
          (set `local.SuccessfullyPickedUpLocal` true))))
    (:`NewEnumerator1`
      ;[1 1 1] Check if we already have one of this weapon type
      (for _array_element_2 (`/Game/Blueprints/Characters/CSCharacter.WeaponInventory` (`self.Character`))
        (bind (_weaponname_2 _weapontype_2 _weaponinstance_2) (break `/Game/Blueprints/Characters/CSWeaponInventory` _array_element_2))
        (if (`|EnumEquality` (`self.WeaponType`) _weapontype_2)
          (`/Engine/EditorBlueprintResources/StandardMacros.IsValid` _weaponinstance_2
            (:`Is Not Valid`
              ;[1 1 1] Create Weapon for character
              (bind _returnvalue (`|SpawnActorFromClass` (`self.PickupWeaponClass`) (`self.GetTransform`) "AlwaysSpawn" "OverrideRootScale" null (`self.Character`)))
              (bind _ascsbase_weapon (cast `/Game/Blueprints/Weapons/CSBaseWeapon` _returnvalue :!pure true))
              (`SceneComponent.SetVisibility` (`/Game/Blueprints/Weapons/CSBaseWeapon.3PP` _ascsbase_weapon) false false)
              ;[1 1 1] Add weapon to inventory
              (`/Game/Blueprints/Characters/CSCharacter.ModifyInventory` (`self.Character`) "NewEnumerator0" "NewEnumerator1" (`self.WeaponType`) _ascsbase_weapon 1)
              ;[1 1 1] Add gratis ammo to inventory
              (`/Game/Blueprints/Characters/CSCharacter.ModifyInventory` (`self.Character`) "NewEnumerator0" "NewEnumerator0" (`self.WeaponType`) null 1)
              (set `local.SuccessfullyPickedUpLocal` true)))))))
  ;[1 1 1] Complete
  (if (`local.SuccessfullyPickedUpLocal`)
    (`GameplayStatics.PlaySoundAtLocation` (`self.PickupSFX`) (`self.K2_GetActorLocation`)))
  (return (`local.SuccessfullyPickedUpLocal`)))

(fn `SetUpPickup`
  (params (PickupType :type "/Game/Blueprints/Ingredients/CSInventoryItemType Enum" :default "NewEnumerator0") (WeaponType :type "/Game/Blueprints/Ingredients/CSAmmoPickupType Enum" :default "NewEnumerator0"))
  (locals (PickupTypeLocal :type "/Game/Blueprints/Ingredients/CSInventoryItemType Enum") (WeaponTypeLocal :type "/Game/Blueprints/Ingredients/CSAmmoPickupType Enum"))
  (bind _weapontypelocal (`local.WeaponTypeLocal`))
  (bind _weapontypelocal_2 (`local.WeaponTypeLocal`))
  (bind _weapontypelocal_3 (`local.WeaponTypeLocal`))
  (set `local.PickupTypeLocal` PickupType)
  (set `local.WeaponTypeLocal` WeaponType)
  (set `self.PickupSFX` (select `/Game/Blueprints/Ingredients/CSInventoryItemType` (`local.PickupTypeLocal`) :`NewEnumerator0` (select `/Game/Blueprints/Ingredients/CSAmmoPickupType` _weapontypelocal_3 :`NewEnumerator0` "/Game/Weapons/AssaultRifle/Audio/Rifle_AmmoPickup_Cue.Rifle_AmmoPickup_Cue" :`NewEnumerator1` "/Game/Weapons/GrenadeLauncher/Audio/GL_AmmoPickup_Cue.GL_AmmoPickup_Cue" :`NewEnumerator3` "/Game/Weapons/RocketLauncher/Audio/RL_AmmoPickup_Cue.RL_AmmoPickup_Cue" :`NewEnumerator4` "/Game/Weapons/Shotgun/Audio/Shotgun_AmmoPickup_Cue.Shotgun_AmmoPickup_Cue" :`NewEnumerator5` "/Game/Weapons/SniperRifle/Audio/SR_AmmoPickup01_Cue.SR_AmmoPickup01_Cue" :!type "SoundBase Object Reference") :`NewEnumerator1` (select `/Game/Blueprints/Ingredients/CSAmmoPickupType` _weapontypelocal_3 :`NewEnumerator0` "/Game/Weapons/AssaultRifle/Audio/Rifle_AmmoPickup_Cue.Rifle_AmmoPickup_Cue" :`NewEnumerator1` "/Game/Weapons/GrenadeLauncher/Audio/GL_AmmoPickup_Cue.GL_AmmoPickup_Cue" :`NewEnumerator3` "/Game/Weapons/RocketLauncher/Audio/RL_AmmoPickup_Cue.RL_AmmoPickup_Cue" :`NewEnumerator4` "/Game/Weapons/Shotgun/Audio/Shotgun_AmmoPickup_Cue.Shotgun_AmmoPickup_Cue" :`NewEnumerator5` "/Game/Weapons/SniperRifle/Audio/SR_AmmoPickup01_Cue.SR_AmmoPickup01_Cue" :!type "SoundBase Object Reference")))
  (`StaticMeshComponent.SetStaticMesh` (`self.PickupMesh`) (select `/Game/Blueprints/Ingredients/CSInventoryItemType` (`local.PickupTypeLocal`) :`NewEnumerator0` (select `/Game/Blueprints/Ingredients/CSAmmoPickupType` _weapontypelocal :`NewEnumerator0` "/Game/Weapons/AssaultRifle/Meshes/Prototype_AssaultRifle_Pickup.Prototype_AssaultRifle_Pickup" :`NewEnumerator1` "/Game/Weapons/GrenadeLauncher/Meshes/Prototype_GrenadeLauncher_Pickup.Prototype_GrenadeLauncher_Pickup" :`NewEnumerator3` "/Game/Weapons/RocketLauncher/Meshes/Prototype_RocketLauncher_Pickup.Prototype_RocketLauncher_Pickup" :`NewEnumerator4` "/Game/Weapons/Shotgun/Meshes/Prototype_Shotgun_Pickup.Prototype_Shotgun_Pickup" :`NewEnumerator5` "/Game/Weapons/SniperRifle/Meshes/Prototype_SniperRifle_Pickup.Prototype_SniperRifle_Pickup" :!type "StaticMesh Object Reference") :`NewEnumerator1` (select `/Game/Blueprints/Ingredients/CSAmmoPickupType` _weapontypelocal :`NewEnumerator0` "/Game/Weapons/AssaultRifle/Meshes/Prototype_AssaultRifle_StaticMesh.Prototype_AssaultRifle_StaticMesh" :`NewEnumerator1` "/Game/Weapons/GrenadeLauncher/Meshes/Prototype_GrenadeLauncher_StaticMesh.Prototype_GrenadeLauncher_StaticMesh" :`NewEnumerator3` "/Game/Weapons/RocketLauncher/Meshes/Prototype_RocketLauncher_StaticMesh.Prototype_RocketLauncher_StaticMesh" :`NewEnumerator4` "/Game/Weapons/Shotgun/Meshes/Prototype_Shotgun_StaticMesh.Prototype_Shotgun_StaticMesh" :`NewEnumerator5` "/Game/Weapons/SniperRifle/Meshes/Prototype_SniperRifle_StaticMesh.Prototype_SniperRifle_StaticMesh" :!type "StaticMesh Object Reference")))
  (switch `/Game/Blueprints/Ingredients/CSInventoryItemType` (`local.PickupTypeLocal`)
    (:`NewEnumerator0`
      ;[1 1 1] Set the clip amount
      (set `self.ClipAmount` (select `/Game/Blueprints/Ingredients/CSAmmoPickupType` (`local.WeaponTypeLocal`) :`NewEnumerator0` 2 :`NewEnumerator1` 2 :`NewEnumerator3` 2 :`NewEnumerator4` 4 :`NewEnumerator5` 1)))
    (:`NewEnumerator1`
      ;[1 1 1] Set up weapon preview
      (set `self.PickupWeaponClass` (select `/Game/Blueprints/Ingredients/CSAmmoPickupType` (`local.WeaponTypeLocal`) :`NewEnumerator0` "/Game/Blueprints/Weapons/CSWeapon_AssaultRifle.CSWeapon_AssaultRifle_C" :`NewEnumerator1` "/Game/Blueprints/Weapons/CSWeapon_GrenadeLauncher.CSWeapon_GrenadeLauncher_C" :`NewEnumerator3` "/Game/Blueprints/Weapons/CSWeapon_RocketLauncher.CSWeapon_RocketLauncher_C" :`NewEnumerator4` "/Game/Blueprints/Weapons/CSWeapon_Shotgun.CSWeapon_Shotgun_C" :`NewEnumerator5` "/Game/Blueprints/Weapons/CSWeapon_SniperRifle.CSWeapon_SniperRifle_C" :!type "Actor Class Reference"))
      (`SceneComponent.K2_SetRelativeLocationAndRotation` (`self.PickupMesh`) (select `/Game/Blueprints/Ingredients/CSAmmoPickupType` _weapontypelocal_2 :`NewEnumerator0` (0.0 -10.0 2.0) :`NewEnumerator1` (0.0 -9.82635 4.015193) :`NewEnumerator3` (0.0 0.0 3.0) :`NewEnumerator4` (0.0 -20.0 2.015193) :`NewEnumerator5` (-0.173649 -9.82635 2.030385) :!type "Vector Structure") (select `/Game/Blueprints/Ingredients/CSAmmoPickupType` _weapontypelocal_2 :`NewEnumerator0` (struct :`Pitch` 90.0) :`NewEnumerator1` (struct :`Pitch` 79.999901 :`Yaw` -89.999878 :`Roll` -89.999878) :`NewEnumerator3` (struct :`Pitch` 80.0) :`NewEnumerator4` (struct :`Pitch` 90.0) :`NewEnumerator5` (struct :`Pitch` 79.999969) :!type "Rotator Structure") false false)))
  ;[1 1 1] Set the dynamic material
  (bind _returnvalue (`PrimitiveComponent.CreateDynamicMaterialInstance` (`self.PickupMesh`) 0 null))
  (set `self.DynamicMaterial` _returnvalue)
  ;[1 1 1] Set the play rate
  (`TimelineComponent.SetPlayRate` (`self.DisolvePickedUpTimeline`) (`self.DisolvePickedUpPlayRate`)))

(fn `UserConstructionScript`
  (`self.SetUpPickup` (`self.PickupType`) (`self.WeaponType`)))