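; Sliding double security door that opens for characters and responds to security-system alarm events.
; A timeline lerps both panels and plays in reverse to close, with sounds and open/closed callbacks.
; The proximity box opens it for CSCharacters and closes it once empty, backed by a looping overlap check and delayed death re-check.
; When connected, alarms close and lock it, recoloring indicator lights through dynamic materials; reset or disabling security unlocks it.
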(event `OpenDoor`
  ;[1 1 1] Open/Close
  (if (and (`self.Closed`) (not (`self.IsLocked`)))
    ;[1 1 1] Set play speed and sfx
    (`TimelineComponent.SetPlayRate` (`self.DoorMovingTimeline`) (`self.DoorOpenPlayRate`))
    (`GameplayStatics.PlaySoundAtLocation` "/Game/Audio/SFX/Ingredients/Blueprints_DoorOpen01_Cue.Blueprints_DoorOpen01_Cue" (`self.K2_GetActorLocation`))
    ;[1 1 1] Open and close animation
    (bind (_direction _dooropenalpha) (`Timeline|DoorMovingTimeline` :!label _label)
      (:`Update`
        (`self.UpdateDoorMovingTimeline` _direction _dooropenalpha))
      (:`Finished`
        (`self.FinishedDoorMovingTimeline` _direction _dooropenalpha)))))

(event `self.ReceiveBeginPlay`
  (`KismetSystemLibrary.K2_SetTimerDelegate` (delegate `CheckOverlappingActors`) (`self.OverlapCheckFrequency`) true))

(event `UpdateDoorMovingTimeline`
  (params (Selection :type "ETimelineDirection Enum" :default "Forward") (DoorOpenAlpha :type "Float (double-precision)"))
  ;[1 1 1] Open and close animation
  (`SceneComponent.K2_SetRelativeLocation` (`self.DoorLeft`) (`KismetMathLibrary.VLerp` (`KismetMathLibrary.MakeVector` (* -1 (.x (`self.DoorOpenTravel`))) (* -1 (.y (`self.DoorOpenTravel`))) (.z (`self.DoorOpenTravel`))) (`self.DoorLeftStart`) DoorOpenAlpha) false false)
  (`SceneComponent.K2_SetRelativeLocation` (`self.DoorRight`) (`KismetMathLibrary.VLerp` (`self.DoorOpenTravel`) (`self.DoorRightStart`) DoorOpenAlpha) false false))

(event `CloseDoor`
  ;[1 1 1] Open/Close
  (if (not (`self.Closed`))
    ;[1 1 1] Set play speed and sfx
    (`TimelineComponent.SetPlayRate` (`self.DoorMovingTimeline`) (`self.DoorClosePlayRate`))
    (`GameplayStatics.PlaySoundAtLocation` "/Game/Audio/SFX/Ingredients/Blueprints_DoorClose01_Cue.Blueprints_DoorClose01_Cue" (`self.K2_GetActorLocation`))
    (goto _label :!via `Reverse`)))

(event `SetLocked`
  (params (NewLocked :type Boolean))
  ;[1 1 1 1 37] Security Events
  (set `self.IsLocked` NewLocked)
  (for _array_element (`self.IndicatorMaterials`)
    (`MaterialInstanceDynamic.SetVectorParameterValue` _array_element "Emissive Tint" (select `bool` (`self.IsLocked`) :`false` (`self.IndicatorColorUnlocked`) :`true` (`self.IndicatorColorLocked`)))))

(event `FinishedDoorMovingTimeline`
  (params (Direction :type "ETimelineDirection Enum" :default "Forward") (DoorOpenAlpha :type "Float (double-precision)"))
  ;[1 1 1] Open and close animation
  (switch `ETimelineDirection` Direction
    (:`Forward`
      (set `self.Closed` false)
      (`self.DoorOpened`))
    (:`Backward`
      (set `self.Closed` true)
      (`self.DoorClosed`))))

(event `/Game/Blueprints/Ingredients/CSSecurityInterface.TripAlarm`
  (params (NewTarget :type "Actor Object Reference"))
  ;[1 1 1 1 37] Security Events
  (set `self.AlarmTrippedLocal` true)
  (if (`self.ConnectedToSecuritySystem`)
    (`self.CloseDoor`)
    (`self.SetLocked` true)))

(event `/Game/Blueprints/Ingredients/CSSecurityInterface.ResetAlarm`
  ;[1 1 1 1 37] Security Events
  (set `self.AlarmTrippedLocal` false)
  (if (`self.ConnectedToSecuritySystem`)
    (`self.SetLocked` false)
    (if (not (`self.UseProximityTrigger`))
      (`self.OpenDoor`))))

(event `/Game/Blueprints/Ingredients/CSSecurityInterface.EnableSecuritySystem`
  ;[1 1 1 1 37] Security Events
  (set `self.SecurityEnabledLocal` true))

(event `/Game/Blueprints/Ingredients/CSSecurityInterface.DisableSecuritySystem`
  ;[1 1 1 1 37] Security Events
  (set `self.SecurityEnabledLocal` false)
  (if (`self.ConnectedToSecuritySystem`)
    (`self.SetLocked` false)
    (`self.OpenDoor`)))

(event `self.ProximityTrigger.OnComponentBeginOverlap`
  (params (OverlappedComponent :type "PrimitiveComponent Object Reference") (OtherActor :type "Actor Object Reference") (OtherComp :type "PrimitiveComponent Object Reference") (OtherBodyIndex :type Integer) (bFromSweep :type Boolean) (SweepResult :type "HitResult Structure (by ref)"))
  ;[1 1 1 1 47] Proximity Trigger
  ;;[1 1 1] If there is a character enters the volume, open the door
  (if (and (and (`self.UseProximityTrigger`) (`self.Closed`)) (not (and (`self.ConnectedToSecuritySystem`) (`self.AlarmTrippedLocal`))))
    (bind _ascscharacter (cast `/Game/Blueprints/Characters/CSCharacter` OtherActor)) ; Open as long as there is a char in the zone
    (`self.OpenDoor`)
    (add `/Game/Blueprints/Characters/CSCharacter.CharacterDied` _ascscharacter (delegate `CharacterDiedInProximityVolume`))))

(event `CharacterDiedInProximityVolume`
  ;[1 1 1 1 47] Proximity Trigger
  ;;[1 1 1] If there is a character enters the volume, open the door
  ;;;[1 1 1] Check Dead
  (`KismetSystemLibrary.RetriggerableDelay` (`/Game/Blueprints/Characters/CSCharacter.DespawnDelay` (stale `self.ProximityTrigger.OnComponentBeginOverlap` _ascscharacter)))
  ;;[1 1 1] When there are no more characters in the volume, close the door
  (if (not (> (`KismetArrayLibrary.Array_Length` (`PrimitiveComponent.GetOverlappingActors` (`self.ProximityTrigger`) "/Game/Blueprints/Characters/CSCharacter.CSCharacter_C")) 0)) :!label _label_2
    (`self.CloseDoor`)))

(event `CheckOverlappingActors`
  ;[1 1 1 1 47] Proximity Trigger
  ;;[1 1 1] Check if we missed anything
  (if (`self.UseProximityTrigger`)
    (goto _label_2)))

(event `self.ProximityTrigger.OnComponentEndOverlap`
  (params (OverlappedComponent :type "PrimitiveComponent Object Reference") (OtherActor :type "Actor Object Reference") (OtherComp :type "PrimitiveComponent Object Reference") (OtherBodyIndex :type Integer))
  ;[1 1 1 1 47] Proximity Trigger
  ;;[1 1 1] When someone leaves, check to see how many are left
  (if (and (and (`self.UseProximityTrigger`) (not (`self.Closed`))) (not (and (`self.ConnectedToSecuritySystem`) (`self.AlarmTrippedLocal`))))
    ;;[1 1 1] When there are no more characters in the volume, close the door
    (cast `Character` OtherActor)
    (goto _label_2)))

(fn `GetAllSecurityIngredients`
  (returns (Ingredients :type "Array of Actor Object Reference"))
  (return (`|MakeArray` null :!type "Actor Object Reference")))

(fn `Scene capture activation`
  (params (Activation :type Boolean))
  (returns (`Capture texture` :type "TextureRenderTarget2D Object Reference"))
  (return null))

(fn `SetAllSecurityIngredients`
  (returns (Return :type Boolean))
  (return false))

(fn `SetFailConditions`
  (params (FailOnAlarmTripped :type Boolean))
  (returns (Return :type Boolean))
  (return false))

(fn `UserConstructionScript`
  (`parent.UserConstructionScript`)
  (`BoxComponent.SetBoxExtent` (`self.ProximityTrigger`) (`self.ProximityTriggerExtent`) true)
  (for _array_element (`|MakeArray` (`self.IndicatorLight1-2`) (`self.IndicatorLight1-3`) (`self.IndicatorLight2-1`) (`self.IndicatorLight2-2`) (`self.IndicatorLight2-3`) (`self.IndicatorLight1-1`))
    (bind _returnvalue (`PrimitiveComponent.CreateDynamicMaterialInstance` _array_element 0 "/Game/Props2/Materials/Emissive_Simple.Emissive_Simple"))
    (`KismetArrayLibrary.Array_Add` (`self.IndicatorMaterials`) _returnvalue))
  (for _array_element_2 (`self.IndicatorMaterials`)
    (`MaterialInstanceDynamic.SetVectorParameterValue` _array_element_2 "Emissive Tint" (select `bool` (`self.IsLocked`) :`false` (`self.IndicatorColorUnlocked`) :`true` (`self.IndicatorColorLocked`)))
    (`MaterialInstanceDynamic.SetScalarParameterValue` _array_element_2 "Emissive Int" (* 15.0 (`self.IndicatorBrightness`))))
  (if (not (`self.Closed`))
    (`TimelineComponent.SetPlaybackPosition` (`self.DoorMovingTimeline`) 1.0 true true)))