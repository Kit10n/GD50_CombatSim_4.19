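; Large security door Blueprint, a child of a door parent class that handles opening, closing and the movement timeline.
; Each timeline update calls the parent, then slides the center door mesh by lerping between its open-travel and start positions with the open alpha.
; The construction script picks one of two gate frame meshes from the Variant setting.
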(event `self.ReceiveBeginPlay`
  (`parent.ReceiveBeginPlay`))

(event `self.ReceiveTick`
  (params (DeltaSeconds :type "Float (single-precision)"))
  (`parent.ReceiveTick` DeltaSeconds))

(event `self.CloseDoor`
  (`parent.CloseDoor`))

(event `self.OpenDoor`
  (`parent.OpenDoor`))

(event `self.UpdateDoorMovingTimeline`
  (params (Selection :type "ETimelineDirection Enum" :default "Forward") (DoorOpenAlpha :type "Float (single-precision)"))
  (`parent.UpdateDoorMovingTimeline` Selection DoorOpenAlpha)
  (`SceneComponent.K2_SetRelativeLocation` (`self.SM_DoorCenter`) (`KismetMathLibrary.VLerp` (`self.CenterOpenTravel`) (`self.CenterStart`) DoorOpenAlpha) false false))

(event `self.FinishedDoorMovingTimeline`
  (params (Direction :type "ETimelineDirection Enum" :default "Forward") (DoorOpenAlpha :type "Float (single-precision)"))
  (`parent.FinishedDoorMovingTimeline` Direction DoorOpenAlpha))

(fn `UserConstructionScript`
  (`parent.UserConstructionScript`)
  (`StaticMeshComponent.SetStaticMesh` (`self.Frame`) (select `int` (`self.Variant`) :`0` "/Game/Environment/Modular/SM_SGate1.SM_SGate1" :`1` "/Game/Environment/Modular/SM_SGate2.SM_SGate2" :!type "StaticMesh Object Reference")))