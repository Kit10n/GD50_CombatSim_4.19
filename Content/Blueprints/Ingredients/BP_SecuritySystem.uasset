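; Security system workstation actor that the game disables when any actor overlaps it.
; On first overlap with the GameInstance's VSecurity at 0, a DoOnce runs a short delayed sequence: button sound, screen mesh swap, GameMode disable message, then VSecurity set to 1.
; If VSecurity is already 1, overlap only applies the changed screen mesh, so the disabled state is read from the GameInstance.
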(event `self.ReceiveActorBeginOverlap`
  (params (OtherActor :type "Actor Object Reference"))
  (bind _ascsgame_instance (cast `/Game/Blueprints/Game/CSGameInstance` (`GameplayStatics.GetGameInstance`)))
  (switch `int` (`/Game/Blueprints/Game/CSGameInstance.V_Security` _ascsgame_instance)
    (:`0`
      (`/Engine/EditorBlueprintResources/StandardMacros.DoOnce` false
        (:`Completed`
          (`KismetSystemLibrary.Delay` 0.2)
          (`GameplayStatics.PlaySound2D` "/Game/Audio/SFX/Ingredients/Blueprints_ButtonPush01_Cue.Blueprints_ButtonPush01_Cue" 5.0)
          (`KismetSystemLibrary.Delay` 0.2)
          (`StaticMeshComponent.SetStaticMesh` (`self.StaticMesh`) "/Game/Props2/SM_Workstation1A_screen6.SM_Workstation1A_screen6")
          (`KismetSystemLibrary.Delay` 0.2)
          (message `/Game/Blueprints/Ingredients/CSSecurityInterface.DisableSecuritySystem` (`GameplayStatics.GetGameMode`))
          (bind _ascsgame_instance_2 (cast `/Game/Blueprints/Game/CSGameInstance` (`GameplayStatics.GetGameInstance`)))
          (set `/Game/Blueprints/Game/CSGameInstance.V_Security` 1 _ascsgame_instance_2))))
    (:`1`
      (`StaticMeshComponent.SetStaticMesh` (`self.StaticMesh`) "/Game/Props2/SM_Workstation1A_screen6.SM_Workstation1A_screen6"))))

(fn `UserConstructionScript`)