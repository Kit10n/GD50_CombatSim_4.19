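; CSAISpawner is a placeable spawner that creates one AI character of a chosen class at its arrow's transform.
; Depending on SpawnType, it fires on BeginPlay or when the player overlaps a linked trigger volume or radius sphere, with all routes sharing a DoOnce.
; After spawning, it stores the character and controller for retrieval and assigns an optional initial patrol path.
; The construction script handles editor visuals and sphere sizing; the preview mesh is destroyed at runtime.
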(event `self.ReceiveBeginPlay`
  ;[1 1 1] Destroy!
  (`ActorComponent.K2_DestroyComponent` (`self.PreviewMesh`))
  (switch `/Game/Blueprints/Ingredients/CSSpawnTypes` (`self.SpawnType`)
    (:`NewEnumerator0`
      (`/Engine/EditorBlueprintResources/StandardMacros.DoOnce` false :!label _label
        (:`Completed`
          (`self.SpawnAI`))))
    (:`NewEnumerator1`
      (add `self.OnActorBeginOverlap` (`self.TriggerVolume`) (delegate `PlayerOverlapsVolume`)))
    (:`NewEnumerator2`
      (`PrimitiveComponent.SetCollisionEnabled` (`self.SphereCollision`) "QueryOnly"))))

(event `PlayerOverlapsVolume` :!signature `self.OnActorBeginOverlap`
  (params (OverlappedActor :type "Actor Object Reference") (OtherActor :type "Actor Object Reference"))
  (cast `/Game/Blueprints/Characters/CSCharacter_Player` OtherActor)
  (goto _label))

(event `self.SphereCollision.OnComponentBeginOverlap`
  (params (OverlappedComponent :type "PrimitiveComponent Object Reference") (OtherActor :type "Actor Object Reference") (OtherComp :type "PrimitiveComponent Object Reference") (OtherBodyIndex :type Integer) (bFromSweep :type Boolean) (SweepResult :type "HitResult Structure (by ref)"))
  (cast `/Game/Blueprints/Characters/CSCharacter_Player` OtherActor)
  (goto _label))

(fn `GetSpawnedAI`
  (returns (SpawnedCharacter :type "/Game/Blueprints/Characters/CSCharacter Object Reference") (SpawnedController :type "/Game/Blueprints/Characters/CSAIController Object Reference"))
  (return (`self.SpawnedCharacter`) (`self.SpawnedController`)))

(fn `SpawnAI`
  (returns (SpawnedCharacter :type "/Game/Blueprints/Characters/CSCharacter Object Reference") (SpawnedController :type "/Game/Blueprints/Characters/CSAIController Object Reference"))
  (bind (_returnvalue_location _returnvalue_rotation) (`KismetMathLibrary.BreakTransform` (`SceneComponent.K2_GetComponentToWorld` (`self.SpawnArrow`))))
  (bind _returnvalue (`AIBlueprintHelperLibrary.SpawnAIFromClass` (`self.CharacterType`) null _returnvalue_location _returnvalue_rotation))
  (bind _output_get (set `self.SpawnedCharacter` (cast `/Game/Blueprints/Characters/CSCharacter` _returnvalue :!pure true)))
  (set `self.SpawnedController` (cast `/Game/Blueprints/Characters/CSAIController` (`Pawn.GetController` _output_get) :!pure true))
  (`/Engine/EditorBlueprintResources/StandardMacros.IsValid` (`self.InitialPatrol`)
    (:`Is Valid`
      (`/Game/Blueprints/Characters/CSAIController.AssignPatrolPath` (`self.SpawnedController`) (`self.InitialPatrol`))
      (set `/Game/Blueprints/Characters/CSCharacter.v_OnAPatrolPath` true (`self.SpawnedCharacter`)))
    (:`Is Not Valid`
      _))
  (return (`self.SpawnedCharacter`) (`self.SpawnedController`)))

(fn `UserConstructionScript`
  ;[1 1 1] #JustSphereThings
  (if (`|EnumEquality` (`self.SpawnType`) "NewEnumerator2")
    (`SceneComponent.SetVisibility` (`self.SphereCollision`) true true)
    (`SphereComponent.SetSphereRadius` (`self.SphereCollision`) (`self.Radius`) true))
  ;[1 1 1] Toggle the raptor
  (if (`KismetSystemLibrary.IsValidClass` (`self.CharacterType`))
    (`SceneComponent.SetVisibility` (`self.Billboard`) false false)
    (`SceneComponent.SetVisibility` (`self.SpawnArrow`) false false)))