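; BP_Database is an actor that switches a screen mesh to a Central Command screen when any actor overlaps it.
; If the game instance's VIsReturning flag is already set, it swaps StaticMesh2 immediately.
; Otherwise, a DoOnce runs a short delayed sequence that plays a button-push sound, swaps the mesh, then sets VIsReturning on the game instance.
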(event `self.ReceiveActorBeginOverlap`
  (params (OtherActor :type "Actor Object Reference"))
  (bind _ascsgame_instance (cast `/Game/Blueprints/Game/CSGameInstance` (`GameplayStatics.GetGameInstance`)))
  (if (`/Game/Blueprints/Game/CSGameInstance.V_IsReturning` _ascsgame_instance)
    (`StaticMeshComponent.SetStaticMesh` (`self.StaticMesh2`) "/Game/Props2/SM_CentralCommandScreenie4.SM_CentralCommandScreenie4")
    (else
      (`/Engine/EditorBlueprintResources/StandardMacros.DoOnce` false
        (:`Completed`
          (`KismetSystemLibrary.Delay` 0.2)
          (`GameplayStatics.PlaySound2D` "/Game/Audio/SFX/Ingredients/Blueprints_ButtonPush01_Cue.Blueprints_ButtonPush01_Cue" 5.0)
          (`KismetSystemLibrary.Delay` 0.2)
          (`StaticMeshComponent.SetStaticMesh` (`self.StaticMesh2`) "/Game/Props2/SM_CentralCommandScreenie4.SM_CentralCommandScreenie4")
          (`KismetSystemLibrary.Delay` 0.2)
          (bind _ascsgame_instance_2 (cast `/Game/Blueprints/Game/CSGameInstance` (`GameplayStatics.GetGameInstance`)))
          (set `/Game/Blueprints/Game/CSGameInstance.V_IsReturning` true _ascsgame_instance_2))))))

(fn `UserConstructionScript`)