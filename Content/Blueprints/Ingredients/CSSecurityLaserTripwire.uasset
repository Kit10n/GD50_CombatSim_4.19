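; Security laser tripwire that trips the game mode alarm and fires WireTripped when a player crosses its beam.
; Construction sizes the collision box and places the receiver from LaserLength, while UpdateBeamLocations aligns the beam particle.
; Toggling follows the security system state, switching visibility and collision, and optionally runs a ping-pong movement timeline with pauses.
; A retriggerable delay re-arms the trigger after the player leaves.
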(event `self.LaserCollision.OnComponentBeginOverlap`
  (params (OverlappedComponent :type "PrimitiveComponent Object Reference") (OtherActor :type "Actor Object Reference") (OtherComp :type "PrimitiveComponent Object Reference") (OtherBodyIndex :type Integer) (bFromSweep :type Boolean) (SweepResult :type "HitResult Structure (by ref)"))
  ;[1 1 1] Overlap event
  (if (and (`self.TripwireEnabled`) (`self.SecuritySystemEnabled`))
    (bind _ascscharacter_player (cast `/Game/Blueprints/Characters/CSCharacter_Player` OtherActor))
    (set `self.TargetInLaser` true)
    (if (not (`self.Triggered`))
      (set `self.Triggered` true)
      (message `/Game/Blueprints/Ingredients/CSSecurityInterface.TripAlarm` (`GameplayStatics.GetGameMode`) _ascscharacter_player)
      (`self.WireTripped` _ascscharacter_player))))

(event `self.ReceiveBeginPlay`
  (`KismetSystemLibrary.Delay` 0.2)
  (bind _ascsgame_mode (cast `/Game/Blueprints/Game/CSGameMode` (`GameplayStatics.GetGameMode`))
    (:`then`
      (bind _output_get (set `self.SecuritySystemEnabled` (`/Game/Blueprints/Game/CSGameMode.SecuritySystemEnabled` _ascsgame_mode))))
    (:`CastFailed`
      (set `self.SecuritySystemEnabled` false)))
  ;[1 1 1] Set beam data
  (`self.ToggleTripwire` (and _output_get (`self.TripwireEnabled`)))
  (`self.UpdateBeamLocations`))

(event `PlayLaserTripwireAnimation`
  (bind _movementstartlocation (`self.MovementStartLocation`))
  ;[1 1 1] Back and forth animation
  (bind (_direction _0_1) (`Timeline|LaserTripwireTimeline` :!label _label)
    (:`Update`
      (`SceneComponent.K2_SetWorldLocation` (`self.SceneRoot`) (`KismetMathLibrary.VLerp` _movementstartlocation (+ _movementstartlocation (`KismetMathLibrary.GreaterGreater_VectorRotator` (`self.MovementEndLocation`) (`self.K2_GetActorRotation`))) _0_1) false false)
      (`self.UpdateBeamLocations`))
    (:`Finished`
      (`KismetSystemLibrary.Delay` (`self.PauseDelay`))
      (switch `ETimelineDirection` _direction
        (:`Forward`
          (`self.ReverseLaserTripwireAnimation`))
        (:`Backward`
          (`self.PlayLaserTripwireAnimation`))))))

(event `self.LaserCollision.OnComponentEndOverlap`
  (params (OverlappedComponent :type "PrimitiveComponent Object Reference") (OtherActor :type "Actor Object Reference") (OtherComp :type "PrimitiveComponent Object Reference") (OtherBodyIndex :type Integer))
  ;[1 1 1] Overlap event
  (if (and (`self.TripwireEnabled`) (`self.SecuritySystemEnabled`))
    (bind _ascscharacter_player (cast `/Game/Blueprints/Characters/CSCharacter_Player` OtherActor))
    (set `self.TargetInLaser` false)
    (`KismetSystemLibrary.RetriggerableDelay` 2.0)
    (if (not (`self.TargetInLaser`))
      (if (`self.Triggered`)
        (set `self.Triggered` false)))))

(event `ReverseLaserTripwireAnimation`
  ;[1 1 1] Back and forth animation
  (goto _label :!via `Reverse`))

(event `ToggleTripwire`
  (params (NewEnabled :type Boolean))
  ;[1 1 1] On/Off
  (bind _output_get (set `self.TripwireEnabled` (select `bool` NewEnabled :`true` true)))
  (`SceneComponent.SetVisibility` (`self.P_LaserTripwire`) _output_get false)
  (`self.UpdateBeamLocations`)
  (`PrimitiveComponent.SetCollisionEnabled` (`self.LaserCollision`) (select `bool` NewEnabled :`false` "NoCollision" :`true` "QueryOnly" :!type "ECollisionEnabled Enum"))
  ;;[1 1 1] Start the anim if it's set to should move
  (if (and NewEnabled (`self.ShouldMove`))
    (`self.PlayLaserTripwireAnimation`)
    (else
      (`TimelineComponent.Stop` (`self.LaserTripwireTimeline`)))))

(event `/Game/Blueprints/Ingredients/CSSecurityInterface.EnableSecuritySystem`
  ;[1 1 1] On/Off
  (bind _output_get (set `self.SecuritySystemEnabled` true))
  (`self.ToggleTripwire` _output_get))

(event `/Game/Blueprints/Ingredients/CSSecurityInterface.DisableSecuritySystem`
  ;[1 1 1] On/Off
  (bind _output_get (set `self.SecuritySystemEnabled` false))
  (`self.ToggleTripwire` _output_get))

(fn `GetAllSecurityIngredients`
  (returns (Ingredients :type "Array of Actor Object Reference"))
  (return))

(fn `Scene capture activation`
  (params (Activation :type Boolean))
  (returns (`Capture texture` :type "TextureRenderTarget2D Object Reference"))
  (return null))

(fn `SetAllSecurityIngredients`
  (returns (Return :type Boolean))
  (return false))

(fn `SetFailConditions`
  (params (FailOnAlarmTripped :type Boolean))
  (returns (Return :type Boolean))
  (return false))

(fn `UpdateBeamLocations`
  (`ParticleSystemComponent.SetBeamSourcePoint` (`self.P_LaserTripwire`) 0 (`SceneComponent.K2_GetComponentLocation` (`self.LaserEmitterBaseMesh`)) 0)
  (`ParticleSystemComponent.SetBeamTargetPoint` (`self.P_LaserTripwire`) 0 (+ (`SceneComponent.K2_GetComponentLocation` (`self.LaserEmitterBaseMesh`)) (* (`KismetMathLibrary.GetForwardVector` (`self.K2_GetActorRotation`)) (.x (`self.LaserEndPosition`)))) 0)
  (return))

(fn `UserConstructionScript`
  ;[1 1 1] Call from construction
  (`parent.UserConstructionScript`)
  ;[1 1 1] Find the laser end pos
  (set `self.LaserEndPosition` (`KismetMathLibrary.MakeVector` (`self.LaserLength`)))
  (set `self.LaserEndPosition` (`KismetMathLibrary.MakeVector` (.x (`self.LaserEndPosition`)) (.y (`SceneComponent.RelativeLocation` (`self.LaserEmitterBaseMesh`))) (.z (`SceneComponent.RelativeLocation` (`self.LaserEmitterBaseMesh`)))))
  ;[1 1 1] Set up laser collision
  (`SceneComponent.K2_SetRelativeLocation` (`self.LaserCollision`) (`KismetMathLibrary.RotateAngleAxis` (`KismetMathLibrary.MakeVector` (`KismetMathLibrary.VSize` (/ (`KismetMathLibrary.Conv_Vector2DToVector` (+ (`KismetMathLibrary.Conv_VectorToVector2D` (`SceneComponent.RelativeLocation` (`self.LaserEmitterBaseMesh`))) (`KismetMathLibrary.Conv_VectorToVector2D` (`self.LaserEndPosition`)))) 2.0)) 0.0 (.z (`SceneComponent.RelativeLocation` (`self.LaserEmitterBaseMesh`)))) 0.0 (0.0 0.0 1.0)) false false)
  ;;[1 1 1] Set Box Extent
  (`BoxComponent.SetBoxExtent` (`self.LaserCollision`) (`KismetMathLibrary.MakeVector` (`KismetMathLibrary.VSize` (/ (`KismetMathLibrary.Conv_Vector2DToVector` (+ (`KismetMathLibrary.Conv_VectorToVector2D` (`SceneComponent.RelativeLocation` (`self.LaserEmitterBaseMesh`))) (`KismetMathLibrary.Conv_VectorToVector2D` (`self.LaserEndPosition`)))) 2.0)) 4.0 4.0) true)
  ;[1 1 1] Set location of end mesh
  (`SceneComponent.K2_SetWorldLocation` (`self.LaserReceiverBaseMesh`) (+ (`SceneComponent.K2_GetComponentLocation` (`self.LaserEmitterBaseMesh`)) (* (`KismetMathLibrary.GetForwardVector` (`self.K2_GetActorRotation`)) (.x (`self.LaserEndPosition`)))) false false)
  ;[1 1 1] Timeline stuff
  (set `self.MovementStartLocation` (`SceneComponent.K2_GetComponentLocation` (`self.SceneRoot`)))
  (`TimelineComponent.SetPlayRate` (`self.LaserTripwireTimeline`) (`self.MovementPlayRate`))
  (`self.UpdateBeamLocations`))