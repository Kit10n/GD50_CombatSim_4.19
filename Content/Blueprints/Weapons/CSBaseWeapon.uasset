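; Base weapon Blueprint for CSCharacter, managing firing, ammo, reloading and equip visuals, with no hit or projectile logic.
; A WeaponState enum and ammo checks gate Fire, which plays audio, VFX, shake and AI noise, then starts a looping timer for automatic refire or cooldown.
; An empty magazine triggers a montage reload that consumes an inventory clip.
; A timeline sweeps a dissolve material's cut plane between muzzle and stock for equip/unequip.
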(event `StartFire`
  ;[1 1 1] Start firing
  (bind (_canfire _shouldreload) (`self.CheckCanFire`))
  (if _canfire
    (`self.Fire`)
    (else
      (`self.StopFire`)
      (if _shouldreload
        (`GameplayStatics.SpawnSoundAttached` "/Game/Weapons/Common/Sound/Weapon_Empty.Weapon_Empty" (`self.K2_GetRootComponent`))
        (`self.StartReload`)))))

(event `PlayDisolveEquipAnimation`
  (params (DestroyWeapon :type Boolean) (PlayRate :type "Float (double-precision)" :default 1.0))
  ;[1 1 1] Equip/unequip disolvefade
  (`TimelineComponent.SetPlayRate` (`self.DisolveEquippedTimeline`) PlayRate)
  (bind (_direction _0_1) (`Timeline|DisolveEquippedTimeline` :!via `PlayFromStart` :!label _label)
    (:`Update`
      (`MaterialInstanceDynamic.SetVectorParameterValue` (`self.DisolveMaterial`) "CutPlane" (`KismetMathLibrary.Conv_VectorToLinearColor` (`KismetMathLibrary.VLerp` (`SceneComponent.GetSocketLocation` (`self.3PP`) (`self.MuzzleFlashSocketName`)) (`SceneComponent.GetSocketLocation` (`self.3PP`) (`self.ButtStockSocketName`)) _0_1)))
      (`MaterialInstanceDynamic.SetVectorParameterValue` (`self.DisolveMaterial`) "CutRotation" (`KismetMathLibrary.Conv_VectorToLinearColor` (`KismetMathLibrary.Conv_RotatorToVector` (`KismetMathLibrary.FindLookAtRotation` (`SceneComponent.GetSocketLocation` (`self.3PP`) (`self.ButtStockSocketName`)) (`SceneComponent.GetSocketLocation` (`self.3PP`) (`self.MuzzleFlashSocketName`)))))))
    (:`Finished`
      (`MaterialInstanceDynamic.SetVectorParameterValue` (`self.DisolveMaterial`) "CutRotation" (`KismetMathLibrary.Conv_VectorToLinearColor` (`KismetMathLibrary.GetUpVector` (struct))))
      (`MaterialInstanceDynamic.SetVectorParameterValue` (`self.DisolveMaterial`) "CutPlane" (`KismetMathLibrary.Conv_VectorToLinearColor` (select `ETimelineDirection` _direction :`Forward` (0.0 0.0 -99999992.0) :`Backward` (0.0 0.0 99999992.0) :!type "Vector Structure")))
      (`TimelineComponent.SetPlayRate` (`self.DisolveEquippedTimeline`) 1.0)
      (if DestroyWeapon
        (`self.K2_DestroyActor`)
        (else
          (set `self.WeaponState` "NewEnumerator0"))))))

(event `StopFire`
  ;[1 1 1] Stop firing
  (`self.Stop`))

(event `ReverseDisolveEquipAnimation`
  (params (PlayRate :type "Float (double-precision)" :default 1.0))
  ;[1 1 1] Equip/unequip disolvefade
  (`TimelineComponent.SetPlayRate` (`self.DisolveEquippedTimeline`) PlayRate)
  (goto _label :!via `ReverseFromEnd`))

(event `StartReload`
  ;[1 1 1] Start reload
  (bind _canreload (`self.CheckCanReload`))
  (if _canreload
    (`self.StopFire`)
    (bind _returnvalue (`self.GetOwnerAnimInstance`))
    (add `AnimInstance.OnMontageEnded` _returnvalue (delegate `FinishedReloading`))
    (bind (_return _returnvalue_2) (`self.Reload`))))

(event `FinishedReloading`
  (params (Montage :type "AnimMontage Object Reference") (bInterrupted :type Boolean))
  (bind _ascscharacter (cast `/Game/Blueprints/Characters/CSCharacter` (`self.CharacterOwner`) :!pure true))
  ;[1 1 1] Finish reload
  (`|ExecutionSequence`
    (:`then_0`
      (if (== (stale `StartReload` _returnvalue_2) Montage)
        (if (not (`/Game/Blueprints/Characters/CSCharacter.InfiniteClips` _ascscharacter))
          (`/Game/Blueprints/Characters/CSCharacter.ModifyInventory` _ascscharacter "NewEnumerator1" "NewEnumerator0" (`self.WeaponType`) null 1))
        (set `self.Ammo` (`self.AmmoMax`))))
    (:`then_1`
      (set `self.WeaponState` "NewEnumerator0")
      (bind _ascscharacter_2 (cast `/Game/Blueprints/Characters/CSCharacter` (`self.GetOwner`)))
      (if (`/Game/Blueprints/Characters/CSCharacter.InputFiring` _ascscharacter_2)
        (`self.StartFire`)))))

(fn `CheckAmmo`
  (returns (HasAmmo :type Boolean) (HasFullAmmo :type Boolean) (HasClips :type Boolean))
  (bind _remainingclips (`self.GetOwnerClips`))
  (return (> (`self.Ammo`) 0) (== (`self.Ammo`) (`self.AmmoMax`)) (> _remainingclips 0)))

(fn `CheckCanFire`
  (returns (CanFire :type Boolean) (ShouldReload :type Boolean))
  (bind _hasammo (`self.CheckAmmo`))
  (bind _output_get (set `self.HasAmmoInClip` _hasammo))
  (return (and _output_get (select `/Game/Blueprints/Weapons/CSWeaponStates` (`self.WeaponState`) :`NewEnumerator0` true :`NewEnumerator1` true) (or (`self.Automatic`) (not (`self.OnCooldown`))) (not (`NavMovementComponent.IsFalling` (`Character.CharacterMovement` (`self.CharacterOwner`))))) (not _hasammo)))

(fn `CheckCanReload`
  (returns (CanReload :type Boolean))
  (bind (_hasammo _hasfullammo _hasclips) (`self.CheckAmmo`))
  (return (and (not _hasfullammo) _hasclips (select `/Game/Blueprints/Weapons/CSWeaponStates` (`self.WeaponState`) :`NewEnumerator0` true :`NewEnumerator1` true))))

(fn `Fire`
  (set `self.WeaponState` "NewEnumerator1")
  (set `self.OnCooldown` true)
  (`self.PlayFireFeedback`)
  (`self.RemoveAmmo`)
  (if (`self.Automatic`)
    (`KismetSystemLibrary.K2_SetTimer` self (`self.AutomaticFunctionName`) (`self.FireRate`) true)
    (else
      (`KismetSystemLibrary.K2_SetTimer` self "OffCooldown" (`self.FireRate`) true))))

(fn `GetAimingMethod`
  (returns (UsingIronsights :type Boolean))
  (locals (UsingIronsightsLocal :type Boolean))
  (bind _ascscharacter (cast `/Game/Blueprints/Characters/CSCharacter` (`self.CharacterOwner`))
    (:`then`
      (set `local.UsingIronsightsLocal` (`/Game/Blueprints/Characters/CSCharacter.InputIronsights` _ascscharacter)))
    (:`CastFailed`
      _))
  (return (`local.UsingIronsightsLocal`)))

(fn `GetOwnerAnimInstance`
  (returns (ReturnValue :type "AnimInstance Object Reference"))
  (bind _ascharacter (cast `Character` (`self.GetInstigator`))
    (:`then`
      _)
    (:`CastFailed`
      _))
  (return (`SkeletalMeshComponent.GetAnimInstance` (`Character.Mesh` _ascharacter))))

(fn `GetOwnerClips`
  (returns (RemainingClips :type Integer))
  (locals (RemainingClipsLocal :type Integer))
  (for _array_element (`/Game/Blueprints/Characters/CSCharacter.WeaponInventory` (cast `/Game/Blueprints/Characters/CSCharacter` (`self.CharacterOwner`) :!pure true))
    (bind (_weaponname _weapontype _weaponinstance _clipscurrent) (break `/Game/Blueprints/Characters/CSWeaponInventory` _array_element))
    (if (`|EnumEquality` (`self.WeaponType`) _weapontype)
      (set `local.RemainingClipsLocal` _clipscurrent)))
  (return (`local.RemainingClipsLocal`)))

(fn `GetWeaponState`
  (returns (WeaponState :type "/Game/Blueprints/Weapons/CSWeaponStates Enum"))
  (return (`self.WeaponState`)))

(fn `OffCooldown`
  (set `self.OnCooldown` false))

(fn `PlayFireFeedback`
  (locals (FireAnimationLocal :type "AnimSequence Object Reference"))
  ;[1 1 1] Weapon animation
  (`SkeletalMeshComponent.PlayAnimation` (`self.3PP`) (`self.WeaponFireAnimation`) false)
  ;[1 1 1] Player animation
  (bind _usingironsights (`self.GetAimingMethod`))
  (set `local.FireAnimationLocal` (select `bool` _usingironsights :`false` (`self.CharacterFireAnimationHips`) :`true` (`self.CharacterFireAnimationIronsights`)))
  ;[1 1 1] VFX
  (`GameplayStatics.SpawnEmitterAttached` (`self.FireVFX`) (`self.3PP`) (`self.MuzzleFlashSocketName`) (0.0 0.0 0.0) (struct) (* (1.0 1.0 1.0) (`self.FireVFXScale`)) "SnapToTargetIncludingScale")
  ;[1 1 1] Automatic or not?
  (if (not (`self.Automatic`))
    ;[1 1 1] Audio
    (`AudioComponent.SetSound` (`self.Audio`) (`self.FireStartSFX`) :!label _label)
    (`AudioComponent.Play` (`self.Audio`) 0.0)
    (set `self.HasPlayedStartFireSFX` true)
    (elif (not (`self.HasPlayedStartFireSFX`))
      (goto _label)
      (elif (!= (`AudioComponent.Sound` (`self.Audio`)) (`self.FireLoopSFX`))
        (`AudioComponent.SetSound` (`self.Audio`) (`self.FireLoopSFX`))
        (`AudioComponent.Play` (`self.Audio`) 0.0))))
  (`AISense_Hearing.ReportNoiseEvent` (`self.K2_GetActorLocation`) 1.0 (`self.GetInstigatorController`))
  ;[1 1 1] Camera Shake
  (bind _ascsplayer_controller (cast `/Game/Blueprints/Characters/CSPlayerController` (`self.GetInstigatorController`))
    (:`then`
      (`PlayerController.ClientStartCameraShake` :`self` _ascsplayer_controller :`Shake` (`self.FireCameraShake`)))
    (:`CastFailed`
      _))
  ;[1 1 1] Force Feedback
  (bind _ascsplayer_controller_2 (cast `/Game/Blueprints/Characters/CSPlayerController` (`self.GetInstigatorController`)))
  (`PlayerController.ClientPlayForceFeedback` _ascsplayer_controller_2 (`self.FireForceFeedback`) false false "None"))

(fn `PlayStopFireFeedback`
  ;[1 1 1] Only if we're an automatic
  (if (`self.Automatic`)
    ;[1 1 1] Audio
    (`AudioComponent.SetSound` (`self.Audio`) (`self.FireStopSFX`))
    (`AudioComponent.Play` (`self.Audio`) 0.0)))

(fn `Reload`
  (returns (Return :type Boolean) (ReturnValue :type "AnimMontage Object Reference"))
  ;[1 1 1] Set the state
  (set `self.WeaponState` "NewEnumerator2")
  ;[1 1 1] Play the animation
  (bind _ascscharacter (cast `/Game/Blueprints/Characters/CSCharacter` (`self.GetInstigator`))
    (:`then`
      (bind _returnvalue (`AnimInstance.PlaySlotAnimationAsDynamicMontage` (`SkeletalMeshComponent.GetAnimInstance` (`Character.Mesh` _ascscharacter)) (`/Game/Blueprints/Characters/CSCharacter.ReloadAnimation` _ascscharacter) "UpperBody" 0.25 0.25 (`self.ReloadPlayRate`) 1 -1.0 0.0)))
    (:`CastFailed`
      _))
  ;[1 1 1] Return
  (return true _returnvalue))

(fn `RemoveAmmo`
  (if (not (`/Game/Blueprints/Characters/CSCharacter.InfiniteAmmo` (cast `/Game/Blueprints/Characters/CSCharacter` (`self.CharacterOwner`) :!pure true)))
    (set `self.Ammo` (`KismetMathLibrary.Clamp` (- (`self.Ammo`) 1) 0 (`self.AmmoMax`)))))

(fn `Stop`
  (`self.GetCurrentState`
    (:`Idle`
      _)
    (:`Firing`
      (set `self.WeaponState` "NewEnumerator0")
      (`KismetSystemLibrary.K2_ClearTimer` self (`self.AutomaticFunctionName`))
      (`self.PlayStopFireFeedback`))
    (:`Reloading`
      _)
    (:`Equiping`
      _))
  (return))

(fn `UserConstructionScript`
  (bind (_handgripoffset_location _handgripoffset_rotation _handgripoffset_scale) (`KismetMathLibrary.BreakTransform` (`self.HandGripOffset`)))
  (bind _3pp (`self.3PP`))
  (bind (_returnvalue_location _returnvalue_rotation) (`KismetMathLibrary.BreakTransform` (`SceneComponent.GetSocketTransform` (`self.3PP`) (`self.GripSocketName`) "RTS_Component")))
  (bind _output_get (set `self.HandGripTransform` (`KismetMathLibrary.MakeTransform` (+ _returnvalue_location _handgripoffset_location) (`KismetMathLibrary.ComposeRotators` _returnvalue_rotation _handgripoffset_rotation) _handgripoffset_scale)))
  (`SceneComponent.K2_SetRelativeLocation` (`self.HandgripLocator`) (.location _output_get) false false)
  ;[1 1 1] Create the dynamic material
  (bind _returnvalue (`PrimitiveComponent.CreateDynamicMaterialInstance` _3pp 0 (`PrimitiveComponent.GetMaterial` _3pp 0)))
  (set `self.DisolveMaterial` _returnvalue)
  ;[1 1 1] Set max ammo
  (set `self.AmmoMax` (`self.Ammo`))
  ;[1 1 1] Timeline
  (`TimelineComponent.SetPlayRate` (`self.DisolveEquippedTimeline`) (`self.DisolveEquipPlayRate`)))