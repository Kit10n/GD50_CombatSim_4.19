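; Projectile weapon Blueprint whose Fire override spawns ProjectileClass actors from the 3PP mesh's MuzzleFlash socket.
; A visibility trace starts at the camera for players or eye height for other characters, ending at the view forward vector times trace distance, without adding the start location.
; Each bullet rotates toward the impact point or trace end, then gets random pitch and yaw spread based on ironsights or hip aiming.
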(fn `Fire`
  (locals (TraceDistanceLocal :type "Float (double-precision)" :default 9999999.0) (ProjectileSpawnRotationLocal :type "Rotator Structure") (TraceStartLocal :type "Vector Structure") (TraceEndLocal :type "Vector Structure") (SpreadLocal :type "Float (double-precision)"))
  (bind _ascscharacter (cast `/Game/Blueprints/Characters/CSCharacter` (`self.GetInstigator`) :!pure true))
  (`parent.Fire`)
  ;[1 1 1] Player or AI firing?
  (cast `/Game/Blueprints/Characters/CSCharacter_Player` (`self.GetInstigator`)
    (:`then`
      (set `local.TraceStartLocal` (`PlayerCameraManager.GetCameraLocation` (`GameplayStatics.GetPlayerCameraManager` 0)))
      (set `local.TraceEndLocal` (* (`SceneComponent.GetForwardVector` (`PlayerCameraManager.TransformComponent` (`GameplayStatics.GetPlayerCameraManager` 0))) (`local.TraceDistanceLocal`))))
    (:`CastFailed`
      (set `local.TraceStartLocal` (`KismetMathLibrary.MakeVector` (.x (`self.K2_GetActorLocation` _ascscharacter)) (.y (`self.K2_GetActorLocation` _ascscharacter)) (+ (.z (`self.K2_GetActorLocation` _ascscharacter)) (`Pawn.BaseEyeHeight` _ascscharacter))))
      (set `local.TraceEndLocal` (* (`self.GetActorForwardVector` (`Pawn.GetController` _ascscharacter)) (`local.TraceDistanceLocal`)))))
  (for _ (range (`self.BulletsPerFire`))
    ;[1 1 1] Where did we shoot?
    (bind _outhit (`KismetSystemLibrary.LineTraceSingle` (`local.TraceStartLocal`) (`local.TraceEndLocal`) "TraceTypeQuery1" true (`|MakeArray` (`self.GetInstigator`) :!type "Actor Object Reference")))
    (bind (_bblockinghit _binitialoverlap _time _distance _location _impactpoint) (`GameplayStatics.BreakHitResult` _outhit))
    ;[1 1 1] Find the delta rotator
    (if _bblockinghit
      (set `local.ProjectileSpawnRotationLocal` (`KismetMathLibrary.FindLookAtRotation` (`SceneComponent.GetSocketLocation` (`self.3PP`) "MuzzleFlash") _impactpoint))
      (else
        (set `local.ProjectileSpawnRotationLocal` (`KismetMathLibrary.FindLookAtRotation` (`SceneComponent.GetSocketLocation` (`self.3PP`) "MuzzleFlash") (`local.TraceEndLocal`)))))
    ;[1 1 1] Spread calcuation
    (bind _usingironsights (`self.GetAimingMethod`))
    (if _usingironsights
      (set `local.SpreadLocal` (`self.IronsightsSpread`))
      (else
        (set `local.SpreadLocal` (`self.HipsSpread`))))
    (set `local.ProjectileSpawnRotationLocal` (`KismetMathLibrary.MakeRotator` (.roll (`local.ProjectileSpawnRotationLocal`)) (+ (.pitch (`local.ProjectileSpawnRotationLocal`)) (`KismetMathLibrary.RandomFloatInRange` (* (`local.SpreadLocal`) -1.0) (`local.SpreadLocal`))) (+ (.yaw (`local.ProjectileSpawnRotationLocal`)) (`KismetMathLibrary.RandomFloatInRange` (* (`local.SpreadLocal`) -1.0) (`local.SpreadLocal`)))))
    ;[1 1 1] Spawn the projectile
    (`|SpawnActorFromClass` (`self.ProjectileClass`) (`KismetMathLibrary.MakeTransform` (`SceneComponent.GetSocketLocation` (`self.3PP`) "MuzzleFlash") (`local.ProjectileSpawnRotationLocal`)) "AlwaysSpawn" "OverrideRootScale" null (`self.GetInstigator`)))
  ;[1 1 1] Return
  (return))

(fn `UserConstructionScript`
  (`parent.UserConstructionScript`))