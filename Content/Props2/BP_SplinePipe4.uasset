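; BP_SplinePipe4 is a prop actor that builds a pipe along an editable spline.
; Its Construction Script loops over each pair of neighboring spline points, adds a spline mesh component per segment and attaches it to TopScene.
; Each segment takes its start and end positions and tangents from the spline in local space, so the pipe follows the curve.
; The event graph holds only disabled placeholder events, with no runtime logic.
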(fn `UserConstructionScript`
  ;[1 1 1] Add pipe meshes to spline and align them
  (for _index (range (+ (- (`SplineComponent.GetNumberOfSplinePoints` (`self.Spline`)) 2) 1))
    (bind _returnvalue (`AddComponent|NODE_AddSplineMeshComponent-1` :`bManualAttachment` true)) ; add new pipe spline mesh component
    (`SceneComponent.K2_AttachTo` _returnvalue (`self.TopScene`) "None" "KeepRelativeOffset" true) ; attach the pipe spline mesh components
    (bind (_location _tangent) (`SplineComponent.GetLocationAndTangentAtSplinePoint` (`self.Spline`) _index "Local"))
    (bind (_location_2 _tangent_2) (`SplineComponent.GetLocationAndTangentAtSplinePoint` (`self.Spline`) (+ _index 1) "Local"))
    (`SplineMeshComponent.SetStartAndEnd` _returnvalue _location _tangent _location_2 _tangent_2 true) ; Update new pipe mesh start/end points\nbased of datas from spline.
  ))